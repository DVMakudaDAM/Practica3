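; Diana is a target Blueprint that scores hits from Dardo (dart) actors.
; When its static mesh is hit, it casts the other actor to Dardo and attaches it to the struck component, keeping its world transform so it sticks in place.
; Each such hit adds a fixed amount to Puntos and writes the new total to a TextRender component.
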(event `self.StaticMesh.OnComponentHit`
  (params (HitComponent :type "PrimitiveComponent Object Reference") (OtherActor :type "Actor Object Reference") (OtherComp :type "PrimitiveComponent Object Reference") (NormalImpulse :type "Vector Structure") (Hit :type "HitResult Structure (by ref)"))
  (bind _asdardo (cast `/Game/Blueprints/Dardo` OtherActor))
  (`self.K2_AttachToComponent` _asdardo HitComponent "None" "KeepWorld" "KeepWorld" "KeepWorld" true)
  (bind _output_get (set `self.Puntos` (+ (`self.Puntos`) 10)))
  (`TextRenderComponent.K2_SetText` (`self.TextRender`) (`KismetTextLibrary.Conv_IntToText` _output_get)))

(fn `UserConstructionScript`)